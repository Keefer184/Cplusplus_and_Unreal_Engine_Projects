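; Third-person player Character with Enhanced Input movement, look, jump, a shoulder-swap camera and simple health.
; Possession adds the input mapping context, and movement follows control yaw only.
; The shoulder-switch action flip-flops a timeline forward and back, lerping the spring arm between left and right offsets, starting left.
; Damage reduces health and destroys the actor at zero; an unconnected flip-flop for jump velocity never runs.
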(event `self.ReceiveAnyDamage`
  (params (Damage :type "Float (single-precision)") (DamageType :type "DamageType Object Reference") (InstigatedBy :type "Controller Object Reference") (DamageCauser :type "Actor Object Reference"))
  (set `self.playerHealth` (- (`self.playerHealth`) Damage))
  (if (<= (`self.playerHealth`) 0.0)
    (`self.K2_DestroyActor`)))

(event `self.ReceivePossessed`
  (params (NewController :type "Controller Object Reference"))
  (bind _asplayer_controller (cast `PlayerController` NewController))
  (`EnhancedInputSubsystemInterface.AddMappingContext` (pcsubsystem `EnhancedInputLocalPlayerSubsystem` _asplayer_controller) "/Game/Input/IM_ThirdPersonCC.IM_ThirdPersonCC" 0 (struct)))

(event `EnhancedInput|/Game/Input/IA_MoveForwardCC`
  (params (ActionValue :type "Float (double-precision)") (ElapsedSeconds :type "Float (double-precision)") (TriggeredSeconds :type "Float (double-precision)") (InputAction :type "InputAction Object Reference" :default "/Game/Input/IA_MoveForwardCC.IA_MoveForwardCC"))
  (:`Triggered`
    (`self.AddMovementInput` (`KismetMathLibrary.GetForwardVector` (`KismetMathLibrary.MakeRotator` 0.0 0.0 (.yaw (`self.GetControlRotation`)))) ActionValue)))

(event `EnhancedInput|/Game/Input/IA_MoveRightCC`
  (params (ActionValue :type "Float (double-precision)") (ElapsedSeconds :type "Float (double-precision)") (TriggeredSeconds :type "Float (double-precision)") (InputAction :type "InputAction Object Reference" :default "/Game/Input/IA_MoveRightCC.IA_MoveRightCC"))
  (:`Triggered`
    (`self.AddMovementInput` (`KismetMathLibrary.GetRightVector` (`KismetMathLibrary.MakeRotator` 0.0 0.0 (.yaw (`self.GetControlRotation`)))) ActionValue)))

(event `EnhancedInput|/Game/Input/IA_TurnCC`
  (params (ActionValue :type "Float (double-precision)") (ElapsedSeconds :type "Float (double-precision)") (TriggeredSeconds :type "Float (double-precision)") (InputAction :type "InputAction Object Reference" :default "/Game/Input/IA_TurnCC.IA_TurnCC"))
  (:`Triggered`
    (`self.AddControllerYawInput` ActionValue)))

(event `EnhancedInput|/Game/Input/IA_LookUpCC`
  (params (ActionValue :type "Float (double-precision)") (ElapsedSeconds :type "Float (double-precision)") (TriggeredSeconds :type "Float (double-precision)") (InputAction :type "InputAction Object Reference" :default "/Game/Input/IA_LookUpCC.IA_LookUpCC"))
  (:`Triggered`
    (`self.AddControllerPitchInput` ActionValue)))

(event `EnhancedInput|/Game/Input/IA_ShoSwitch`
  (params (ActionValue :type Boolean) (ElapsedSeconds :type "Float (double-precision)") (TriggeredSeconds :type "Float (double-precision)") (InputAction :type "InputAction Object Reference" :default "/Game/Input/IA_ShoSwitch.IA_ShoSwitch"))
  (:`Triggered`
    (`/Engine/EditorBlueprintResources/StandardMacros.FlipFlop`
      (:`A`
        (bind (_direction _camlocblendalpha) (`Timeline|T_ShoSwitch` :!label _label)
          (:`Update`
            (`SceneComponent.K2_SetRelativeLocation` (`self.ShoulderSpringArm`) (`KismetMathLibrary.VLerp` (`self.LShoCamLoc`) (`self.RShoCamLoc`) _camlocblendalpha) false false))))
      (:`B`
        (goto _label :!via `Reverse`)))))

(event `EnhancedInput|/Game/Input/IA_Jump`
  (params (ActionValue :type Boolean) (ElapsedSeconds :type "Float (double-precision)") (TriggeredSeconds :type "Float (double-precision)") (InputAction :type "InputAction Object Reference" :default "/Game/Input/IA_Jump.IA_Jump"))
  (:`Triggered`
    (`self.Jump`)))

(fn `UserConstructionScript`
  (`SceneComponent.K2_SetRelativeLocation` (`self.ShoulderSpringArm`) (`self.LShoCamLoc`) false false))