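; BP_JumpBoost is a pickup that temporarily changes the jump velocity of a BP_CharacterController that overlaps its box.
; On overlap it sets the character's JumpZVelocity to JumpVelocity, toggles the JumpBoost component's visibility and disables box collision.
; A single CoolDownTime delay serves as both effect duration and respawn time, after which visibility and collision return and JumpZVelocity resets to a hardcoded default.
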(event `self.Box.OnComponentBeginOverlap`
  (params (OverlappedComponent :type "PrimitiveComponent Object Reference") (OtherActor :type "Actor Object Reference") (OtherComp :type "PrimitiveComponent Object Reference") (OtherBodyIndex :type Integer) (bFromSweep :type Boolean) (SweepResult :type "HitResult Structure (by ref)"))
  (bind _asbp_character_controller (cast `/Game/BP/BP_CharacterController` OtherActor))
  (bind _charactermovement (`Character.CharacterMovement` _asbp_character_controller))
  (set `CharacterMovementComponent.JumpZVelocity` (`self.jumpVelocity`) _charactermovement)
  (`SceneComponent.ToggleVisibility` (`self.JumpBoost`) false)
  (`PrimitiveComponent.SetCollisionEnabled` (`self.Box`) "NoCollision")
  (`KismetSystemLibrary.Delay` (`self.coolDownTime`))
  (`SceneComponent.ToggleVisibility` (`self.JumpBoost`) false)
  (`PrimitiveComponent.SetCollisionEnabled` (`self.Box`) "QueryAndPhysics")
  (`/Engine/EditorBlueprintResources/StandardMacros.IsValid` _asbp_character_controller
    (:`Is Valid`
      (set `CharacterMovementComponent.JumpZVelocity` 600.0 _charactermovement))))

(fn `UserConstructionScript`)