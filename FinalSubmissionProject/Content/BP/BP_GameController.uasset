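; Game controller Blueprint that creates the HUD and respawns the player when their character is destroyed.
; On BeginPlay it adds W_Hud to the viewport, caches a PlayerStart transform as the spawn point, and binds to the player character's OnDestroyed.
; On destruction it spawns a BP_CharacterController there, has the player controller possess it, and calls Respawn to rebind the event for the next death.
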(event `self.ReceiveBeginPlay`
  (`|ExecutionSequence`
    (:`then_0`
      (bind _returnvalue (`|CreateWidget` "/Game/UI/W_Hud.W_Hud_C"))
      (bind _output_get (set `self.Hud_Ref` _returnvalue))
      (`UserWidget.AddToViewport` _output_get 0))
    (:`then_1`
      (bind _returnvalue_2 (`GameplayStatics.GetActorOfClass` "/Script/Engine.PlayerStart"))
      (set `self.spawnLocation` (`self.GetTransform` _returnvalue_2)))
    (:`then_2`
      (add `self.OnDestroyed` (`GameplayStatics.GetPlayerCharacter` 0) (delegate `OnDestroyed_Event`) :!label _label))))

(event `Respawn`
  (goto _label))

(event `OnDestroyed_Event` :!signature `self.OnDestroyed`
  (params (DestroyedActor :type "Actor Object Reference"))
  (bind _returnvalue (`|SpawnActorFromClass` "/Game/BP/BP_CharacterController.BP_CharacterController_C" (`self.spawnLocation`) "Undefined" "MultiplyWithRoot" null null))
  (`Controller.Possess` (`GameplayStatics.GetPlayerController` 0) _returnvalue)
  (`self.Respawn`))

(fn `UserConstructionScript`)